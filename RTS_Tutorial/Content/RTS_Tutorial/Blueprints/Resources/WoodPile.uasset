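; WoodPile is a resource actor that hands wood to nearby NPCs in an RTS tutorial project.
; Every Tick it gets all NPC_BP actors and, for each within 400 units, moves one unit of its Wood to that NPC, up to the NPC's MaxWood.
; The transfer rate follows frame rate, the pile's own Wood has no depletion check, and a debug string prints for each NPC in range.
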(event `self.ReceiveTick`
  (params (DeltaSeconds :type "Float (single-precision)"))
  (bind _outactors (`GameplayStatics.GetAllActorsOfClass` "/Game/RTS_Tutorial/Blueprints/AI/NPC_BP.NPC_BP_C"))
  (for _array_element _outactors
    (if (< (`KismetMathLibrary.VSize` (- (`self.K2_GetActorLocation` _array_element) (`self.K2_GetActorLocation`))) 400.0)
      (bind _returnvalue (+ (`/Game/RTS_Tutorial/Blueprints/AI/NPC_BP.Wood` _array_element) 1))
      (`KismetSystemLibrary.PrintString` (`KismetStringLibrary.Conv_IntToString` _returnvalue))
      (if (<= _returnvalue (`/Game/RTS_Tutorial/Blueprints/AI/NPC_BP.MaxWood` _array_element))
        (set `/Game/RTS_Tutorial/Blueprints/AI/NPC_BP.Wood` _returnvalue _array_element)
        (`/Engine/EditorBlueprintResources/StandardMacros.DecrementInt` (`self.Wood`))))))

(fn `UserConstructionScript`)