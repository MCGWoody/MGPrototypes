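; ConstructionProxy_BP is a ghost-material placeholder for a building under construction, with mesh, entrance and collision box set up in the construction script.
; Workers join through ReportToShift, and each Tick advances a clockwork timer using the game-speed time unit divided by worker count.
; Once work time reaches the required construction time, it fires ConstructionCompleted, frees and unhides its workers, and destroys itself after a short delay.
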(event `self.ReceiveBeginPlay`
  (`KismetSystemLibrary.PrintString` "proxy spawned")
  (bind _output_get (set `self.GameStateRef` (cast `/Game/RTS_Tutorial/GameBP/MyGameState` (`GameplayStatics.GetGameState`) :!pure true)))
  (add `/Game/RTS_Tutorial/GameBP/MyGameState.UpdateGameSpeed` _output_get (`|CreateDelegate` :!event `AdjustTime`))
  (bind _timeunit (`/Game/RTS_Tutorial/GameBP/MyGameState.GetCurrentTimeUnit` (`self.GameStateRef`)))
  (set `self.TimeUnit` _timeunit))

(event `self.ReceiveTick`
  (params (DeltaSeconds :type "Float (single-precision)"))
  (set `self.Delta` DeltaSeconds)
  (if (not (`self.IsConstructionCompleted`))
    (`self.DoWork`)
    (if (>= (`self.WorkTimeSpent`) (`self.ConstructionTime`))
      (set `self.IsConstructionCompleted` true)
      (`self.ConstructionCompleted` self)
      (`self.ConstructionComplete`)
      (`KismetSystemLibrary.Delay` 0.2)
      (`self.K2_DestroyActor`))))

(event `AdjustTime`
  (params (TimeUnit :type "Float (double-precision)"))
  (set `self.TimeUnit` TimeUnit))

(fn `ConstructionComplete`
  (if (> (`self.GetWorkForce`) 0.0)
    (for _array_element (`self.ActiveWorkers`)
      (`/Game/RTS_Tutorial/Blueprints/AI/NPC_BP.SetIsBusy` _array_element false)
      (`self.SetActorHiddenInGame` _array_element false))
    (set `self.ActiveWorkers` (`|MakeArray` null :!type "/Game/RTS_Tutorial/Blueprints/AI/NPC_BP Object Reference"))
    (return)
    (else
      (return))))

(fn `DoWork`
  (bind _activeworkers (`self.GetWorkForce`))
  (if (> _activeworkers 0.0)
    (bind _output_get (set `self.Clockwork` (`/Game/RTS_Tutorial/Libraries/FunctionLibrary.SetClockwork` (`self.Delta`) (/ (`self.TimeUnit`) _activeworkers) (`self.Clockwork`))))
    (set `self.WorkTimeSpent` (* _output_get 60.0))
    (return)
    (else
      (return))))

(fn `GetWorkForce`
  (returns (ActiveWorkers :type "Float (double-precision)"))
  (return (`KismetMathLibrary.Conv_IntToDouble` (`KismetArrayLibrary.Array_Length` (`self.ActiveWorkers`)))))

(fn `ReportToShift`
  (params (Worker :type "/Game/RTS_Tutorial/Blueprints/AI/NPC_BP Object Reference"))
  (`KismetArrayLibrary.Array_Add` (`self.ActiveWorkers`) Worker)
  (return))

(fn `SetConstructionTime`
  (params (WorkHours :type "Float (double-precision)"))
  (set `self.ConstructionTime` (* WorkHours 60.0))
  (return))

(fn `UserConstructionScript`
  (bind _staticmesh (`self.StaticMesh`))
  (`StaticMeshComponent.SetStaticMesh` _staticmesh (`self.DisplayMesh`))
  (`PrimitiveComponent.SetMaterial` _staticmesh 0 "/Game/RTS_Tutorial/Materials/GhostConstruct_M_Inst3.GhostConstruct_M_Inst3")
  (`/Game/RTS_Tutorial/Libraries/FunctionLibrary.SetBuildingEntrance` (`self.Entrance`) (`self.StaticMesh`))
  (`/Game/RTS_Tutorial/Libraries/FunctionLibrary.SetBuildingCollisionBox` (`self.Collision`) (`self.StaticMesh`)))