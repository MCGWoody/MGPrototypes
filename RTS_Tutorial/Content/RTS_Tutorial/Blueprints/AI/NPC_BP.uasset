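; RTS villager NPC that gets a random identity and is driven by an NPC_AIController.
; The construction script picks a random sex, tints a dynamic body material to match, draws a name from per-sex enums, then stores and prints it.
; BeginPlay caches the controller for SetIsBusy's blackboard write, and GetClosestActor provides a nearest-actor search.
; Tick fetches all WoodPile actors every frame but leaves the result unused.
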(event EventBeginPlay
  (bind _returnvalue (AI|GetAIController self))
  (Variables|References|SetAIControllerRef (.AsNPC%20AIController (Utilities|Casting|CastToNPC_AIController _returnvalue))))

(event EventActorBeginOverlap
  (params (OtherActor :type Actor%20Object%20Reference)))

(event EventTick
  (params (DeltaSeconds :type Float%20%28single-precision%29))
  (bind _outactors (Actor|GetAllActorsOfClass "/Game/RTS_Tutorial/Blueprints/Resources/WoodPile.WoodPile_C")))

(fn ConstructionScript
  (CallFunction|RandomNPCFeatures))

(fn RandomNPCFeatures
  (bind _returnvalue (Rendering|Material|CreateDynamicMaterialInstance (Variables|Character|GetMesh) 0 "/Game/RTS_Tutorial/Character/Materials/M_UE4Man_Body_Inst.M_UE4Man_Body_Inst" :!class /Script/Engine.PrimitiveComponent))
  (LocalVariables|SetMaterialInstance _returnvalue)
  (if (Utilities|Enum|Equal(Enum) (Utilities|Enum|LiteralenumNPCSex_ENUM (Utilities|Enum|ByteToEnumNPCSex_ENUM (Math|Conversions|ToByte(Integer) (Math|Random|RandomIntegerinRange 0 1)))) "NewEnumerator0")
    (Rendering|Material|SetVectorParameterValue (LocalVariables|GetMaterialInstance) "BodyColor" (LocalVariables|GetMaleColor) :!class /Script/Engine.MaterialInstanceDynamic)
    (bind _name (CallFunction|GetRandomName "NewEnumerator0"))
    (Variables|Default|SetMyProfile (Utilities|Struct|MakeNPCProfile_Struct _name "NewEnumerator0"))
    (Development|PrintString _name)
    (else
      (Rendering|Material|SetVectorParameterValue (LocalVariables|GetMaterialInstance) "BodyColor" (LocalVariables|GetFemaleColor) :!class /Script/Engine.MaterialInstanceDynamic)
      (bind _name_2 (CallFunction|GetRandomName "NewEnumerator1"))
      (Variables|Default|SetMyProfile (Utilities|Struct|MakeNPCProfile_Struct _name_2 "NewEnumerator1"))
      (Development|PrintString _name_2))))

(fn GetRandomName
  (params (Sex :type NPCSex_ENUM%20Enum))
  (if (Utilities|Enum|Equal(Enum) Sex "NewEnumerator0")
    (return (Utilities|String|EnumtoString (Utilities|Enum|LiteralenumNPCNameMale_ENUM (Utilities|Enum|ByteToEnumNPCNameMale_ENUM (Math|Conversions|ToByte(Integer) (Math|Random|RandomIntegerinRange 0 (- (|GetNumEnumEntries) 1)))))))
    (else
      (return (Utilities|String|EnumtoString (Utilities|Enum|LiteralenumNPCNameFemale_ENUM (Utilities|Enum|ByteToEnumNPCNameFemale_ENUM (Math|Conversions|ToByte(Integer) (Math|Random|RandomIntegerinRange 0 (- (|GetNumEnumEntries) 1))))))))))

(fn SetIsBusy
  (params (IsBusy :type Boolean))
  (AI|Components|Blackboard|SetValueasBool (AI|GetBlackboard (Variables|References|GetAIControllerRef)) (Variables|Default|GetIsBusy) IsBusy)
  (return))

(fn GetClosestActor
  (params (Actors :type Array%20of%20Actor%20Object%20References))
  (for _array_element Actors
    (if (or (< (Math|Vector|VectorLength (- (Transformation|GetActorLocation) (Transformation|GetActorLocation _array_element))) (LocalVariables|Getdist)) (< (LocalVariables|Getdist) 0.0))
      (LocalVariables|Setreturn _array_element)
      (LocalVariables|Setdist (Math|Vector|VectorLength (- (Transformation|GetActorLocation) (Transformation|GetActorLocation _array_element))))))
  (return (LocalVariables|Getreturn)))